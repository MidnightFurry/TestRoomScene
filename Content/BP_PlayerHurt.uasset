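; BP_PlayerHurt is a hazard that damages the player while they overlap its owning actor.
; Each Tick it checks that overlap, casts the player to BP_ThirdPersonCharacter, plays a world camera shake at the owner and applies fixed damage.
; Damage repeats every frame without cooldown or delta-time scaling, and the result is printed for debugging.
; BeginPlay zeroes a Shakadeescaly variable that the Tick logic never uses.
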(event `self.ReceiveBeginPlay`
  (set `self.shakadeescaly` 0))

(event `self.ReceiveTick`
  (params (DeltaSeconds :type "Float (single-precision)"))
  (bind _returnvalue (`self.GetOwner`))
  (if (`Actor.IsOverlappingActor` _returnvalue (`GameplayStatics.GetPlayerCharacter` 0))
    (bind _asbp_third_person_character (cast `/Game/ThirdPerson/Blueprints/BP_ThirdPersonCharacter` (`GameplayStatics.GetPlayerCharacter` 0)))
    (`GameplayStatics.PlayWorldCameraShake` "/Script/Engine.CameraShakeBase" (`Actor.K2_GetActorLocation` _returnvalue) 0.0 800.0)
    (bind _returnvalue_2 (`GameplayStatics.ApplyDamage` _asbp_third_person_character 5.0))
    (`KismetSystemLibrary.PrintString` (`KismetStringLibrary.Conv_DoubleToString` _returnvalue_2) true true (struct :`G` 0.66 :`B` 1.0 :`A` 1.0) 2.0 "4")))